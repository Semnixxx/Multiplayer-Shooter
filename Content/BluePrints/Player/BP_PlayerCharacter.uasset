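; Player character Blueprint that handles movement, looking, jumping and weapon use through a BPWeaponManager.
; On possession, the authority creates a rifle through the manager and selects it.
; Fire press and release go through server events to start or stop using the current weapon.
; Reload input checks that the current weapon is a BP_FireWeapon, then a server event sets its Reloading flag.
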(event Custom|Server_Fire
  (params (Active :type Boolean))
  (bind _bp_weaponmanager (Variables|Components|GetBP_WeaponManager))
  (bind _currentweapon (Variables|/Game/BluePrints/Components/Player/BP_WeaponManager.BP_WeaponManager_C|GetCurrentWeapon _bp_weaponmanager))
  ;[1 0.09351 0.1134] Fire from Weapon and Reloading
  (if Active
    (Default|UseWeapon _currentweapon)
    (else
      (Default|StopUseWeapon _currentweapon))))

(event Custom|ServerReloadWeapon
  ;[1 0.09351 0.1134] Fire from Weapon and Reloading
  (bind _asbp_fire_weapon (Utilities|Casting|CastToBP_FireWeapon (Variables|/Game/BluePrints/Components/Player/BP_WeaponManager.BP_WeaponManager_C|GetCurrentWeapon (Variables|Components|GetBP_WeaponManager))))
  (Variables|/Game/BluePrints/Weapons/BP_FireWeapon.BP_FireWeapon_C|SetReloading _asbp_fire_weapon true))

(event EventPossessed
  (params (NewController :type Controller%20Object%20Reference))
  (bind _bp_weaponmanager (Variables|Components|GetBP_WeaponManager))
  ;[1 1 1] Test
  (Networking|SwitchHasAuthority
    (:Authority
      (bind _weapon (Default|CreateWeapon _bp_weaponmanager "/Game/BluePrints/Weapons/BP_Weapon_Rifle.BP_Weapon_Rifle_C"))
      (Default|SelectWeapon _bp_weaponmanager _weapon))))

(event Input|ActionEvents|InputActionFire
  (params (Key :type Key%20Structure :default "None"))
  ;[1 0.09351 0.1134] Fire from Weapon and Reloading
  (:Pressed
    (CallFunction|ServerFire true))
  (:Released
    (CallFunction|ServerFire false)))

(event Input|ActionEvents|InputActionJump
  (params (Key :type Key%20Structure :default "None"))
  ;[0.004132 0.3801 1] Movement
  (:Pressed
    (Character|Jump)))

(event Input|ActionEvents|InputActionReload
  (params (Key :type Key%20Structure :default "None"))
  ;[1 0.09351 0.1134] Fire from Weapon and Reloading
  (:Pressed
    (Utilities|Casting|CastToBP_FireWeapon (Variables|/Game/BluePrints/Components/Player/BP_WeaponManager.BP_WeaponManager_C|GetCurrentWeapon (Variables|Components|GetBP_WeaponManager)))
    (CallFunction|ServerReloadWeapon)))

(event Input|AxisEvents|InputAxisLookUp
  (params (AxisValue :type Float%20%28single-precision%29))
  ;[0.004132 0.3801 1] Loock Around
  (Pawn|Input|AddControllerPitchInput AxisValue))

(event Input|AxisEvents|InputAxisTurn
  (params (AxisValue :type Float%20%28single-precision%29))
  ;[0.004132 0.3801 1] Loock Around
  (Pawn|Input|AddControllerYawInput AxisValue))

(event Input|AxisEvents|InputAxisMoveForward
  (params (AxisValue :type Float%20%28single-precision%29))
  ;[0.004132 0.3801 1] Movement
  (Pawn|Input|AddMovementInput (Transformation|GetActorForwardVector) AxisValue false))

(event Input|AxisEvents|InputAxisMoveRight
  (params (AxisValue :type Float%20%28single-precision%29))
  ;[0.004132 0.3801 1] Movement
  (Pawn|Input|AddMovementInput (Transformation|GetActorRightVector) AxisValue false))

(fn ConstructionScript)